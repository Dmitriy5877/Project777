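; BP_Button is an interactable switch that shows a UI when a character is nearby and can toggle a set of lights.
; Entering its Box creates a WBP_ButtonUI widget, passes it a button reference and sets Game and UI input; leaving removes the widget but keeps that input mode.
; ToggleSwitch flips root component visibility on each actor in the Lights array, with no caller in this Blueprint.
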(event `self.Box.OnComponentBeginOverlap`
  (params (OverlappedComponent :type "PrimitiveComponent Object Reference") (OtherActor :type "Actor Object Reference") (OtherComp :type "PrimitiveComponent Object Reference") (OtherBodyIndex :type Integer) (bFromSweep :type Boolean) (SweepResult :type "HitResult Structure (by ref)"))
  (cast `Character` OtherActor)
  (set `self.bPlayerInRange` true)
  (bind _returnvalue (`|CreateWidget` "/Game/Blieprints/WBP_ButtonUI.WBP_ButtonUI_C" null (`self.ButtonReference`)))
  (`UserWidget.AddToViewport` _returnvalue 0)
  (`WidgetBlueprintLibrary.SetInputMode_GameAndUIEx` (`GameplayStatics.GetPlayerController` 0) null "DoNotLock" false))

(event `self.Box.OnComponentEndOverlap`
  (params (OverlappedComponent :type "PrimitiveComponent Object Reference") (OtherActor :type "Actor Object Reference") (OtherComp :type "PrimitiveComponent Object Reference") (OtherBodyIndex :type Integer))
  (cast `Character` OtherActor)
  (set `self.bPlayerInRange` false)
  (`Widget.RemoveFromParent` (stale `self.Box.OnComponentBeginOverlap` _returnvalue)))

(event `ToggleSwitch`
  (for _array_element (`self.Lights`)
    (`SceneComponent.ToggleVisibility` (`Actor.RootComponent` _array_element) false)))

(fn `UserConstructionScript`)